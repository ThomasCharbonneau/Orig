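; Battle simulator that resolves one round of turn-based monster combat between the player's monster and an opponent.
; SimulateRound orders attacks by Speed with random tie-breaks, picks a random opponent move, and skips the slower monster's attack if it has died.
; ProcessMove scales physical or magical damage by attack over defense, rolls criticals and subtracts health.
; Each move updates combat text, then CombatUI receives turn end; its delay calls are unwired.
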(event Custom|Simulate%20Round
  (params (Player%20Monster :type Monster%20Object%20Reference%20%28by%20ref%29) (Opponent%20Monster :type Monster%20Object%20Reference%20%28by%20ref%29) (Player%20Selected%20Move :type Moves%20Object%20Reference%20%28by%20ref%29) (CombatUI :type Combat%20UI%20Object%20Reference))
  (bind _moveset_ (Variables|/Script/Orig.Monster|GetmoveSet_ Opponent%20Monster))
  (bind _moves_ (Variables|/Script/Orig.MoveSet|Getmoves_ _moveset_))
  (bind _outitem (Utilities|Array|Random _moves_))
  ;[1 1 1] Determine which monster is faster
  (if (== (Variables|/Script/Orig.MonsterStats|Getspeed_ (Variables|/Script/Orig.Monster|Getstats_ Player%20Monster)) (Variables|/Script/Orig.MonsterStats|Getspeed_ (Variables|/Script/Orig.Monster|Getstats_ Opponent%20Monster)))
    (if (== 0 (Math|Conversions|ToInteger(Byte) (Class|KismetMathLibrary|RandomInteger64inRange 0 1)))
      (Variables|Default|SetFastest%20Monster Player%20Monster :!label _label)
      (Variables|Default|SetFastest%20Moves Player%20Selected%20Move)
      (Variables|Default|SetSlowest%20Monster Opponent%20Monster)
      (Variables|Default|SetSlowest%20Moves _outitem)
      (else
        (Variables|Default|SetFastest%20Monster Opponent%20Monster :!label _label_2)
        (Variables|Default|SetFastest%20Moves _outitem)
        (Variables|Default|SetSlowest%20Monster Player%20Monster)
        (Variables|Default|SetSlowest%20Moves Player%20Selected%20Move)))
    (elif (> (Variables|/Script/Orig.MonsterStats|Getspeed_ (Variables|/Script/Orig.Monster|Getstats_ Player%20Monster)) (Variables|/Script/Orig.MonsterStats|Getspeed_ (Variables|/Script/Orig.Monster|Getstats_ Opponent%20Monster)))
      (goto _label)
      (else
        (goto _label_2))))
  (CallFunction|ProcessMove (Variables|Default|GetFastest%20Monster) (Variables|Default|GetSlowest%20Monster) (Variables|Default|GetFastest%20Moves))
  (Default|SetCombatText (Variables|Default|GetCombatTextBp) (Utilities|Text|ToText(String) (Utilities|String|Append (Variables|/Script/Orig.Moves|Getname (Variables|Default|GetFastest%20Moves)) (Utilities|String|Append (Variables|/Script/Orig.Monster|Getname (Variables|Default|GetFastest%20Monster)) " used "))))
  (bind _returnvalue (Class|Monster|IsAlive (Variables|Default|GetSlowest%20Monster)))
  (if _returnvalue
    (CallFunction|ProcessMove (Variables|Default|GetSlowest%20Monster) (Variables|Default|GetFastest%20Monster) (Variables|Default|GetSlowest%20Moves))
    (Default|SetCombatText (Variables|Default|GetCombatTextBp) (Utilities|Text|ToText(String) (Utilities|String|Append (Variables|/Script/Orig.Moves|Getname (Variables|Default|GetSlowest%20Moves)) (Utilities|String|Append (Variables|/Script/Orig.Monster|Getname (Variables|Default|GetSlowest%20Monster)) " used ")))))
  (Default|CombatTurnEnded CombatUI Player%20Monster Opponent%20Monster))

(event Custom|On%20Initialization
  (params (CombatTextBlueprint :type Combat%20Text%20Blueprint%20Object%20Reference) (CombatUI :type Combat%20UI%20Object%20Reference))
  (bind _returnvalue (Game|ConstructObjectfromClass "/Script/Orig.BattleSimulation" self))
  (Variables|Default|SetBattle%20Simulation _returnvalue)
  (Variables|Default|SetCombatTextBp CombatTextBlueprint)
  (Variables|Default|SetCombatUI CombatUI))

(fn ProcessMove
  (params (Attacker :type Monster%20Object%20Reference%20%28by%20ref%29) (Receiver :type Monster%20Object%20Reference%20%28by%20ref%29) (Move :type Moves%20Object%20Reference%20%28by%20ref%29))
  (bind _stats_ (Variables|/Script/Orig.Monster|Getstats_ Receiver))
  (bind _damage (Variables|/Script/Orig.Moves|Getdamage Move))
  (bind _stats__2 (Variables|/Script/Orig.Monster|Getstats_ Attacker))
  (bind _stats__3 (Variables|/Script/Orig.Monster|Getstats_ Attacker))
  (bind _returnvalue (Math|Conversions|ToInteger(Byte) _damage))
  (bind _returnvalue_2 (Math|Conversions|ToFloat(Integer) _returnvalue))
  ;[1 1 1] Apply damage and defense based on damage type
  (switch Utilities|FlowControl|Switch|SwitchonEAttackTypes (Variables|/Script/Orig.Moves|GetDamageType Move)
    (:Physical
      (Variables|Default|SetDamage%20Dealt (Math|Conversions|ToInteger(Byte) (Class|KismetMathLibrary|Round64 (* (Variables|/Script/Orig.MonsterStats|GetphysicalDamage_ _stats__3) (/ _returnvalue_2 (Variables|/Script/Orig.MonsterStats|GetphysicalDefense_ _stats_)))))))
    (:Magical
      (Variables|Default|SetDamage%20Dealt (Math|Conversions|ToInteger(Byte) (Class|KismetMathLibrary|Round64 (* (Variables|/Script/Orig.MonsterStats|GetmagicDamage_ _stats__3) (/ _returnvalue_2 (Variables|/Script/Orig.MonsterStats|GetmagicDefense_ _stats_))))))))
  ;[1 1 1] Apply critical strike based on critical chance
  (if (< (Math|Random|RandomInteger 100) (Variables|/Script/Orig.MonsterStats|GetcriticalChance_ _stats__2))
    (Variables|Default|SetDamage%20Dealt (Math|Float|Round (* (Variables|Default|GetDamage%20Dealt) (Variables|/Script/Orig.MonsterStats|GetcriticalDamage_ _stats__2)))))
  (Variables|/Script/Orig.MonsterStats|SetcurrentHealth_ _stats_ (- (Variables|/Script/Orig.MonsterStats|GetcurrentHealth_ _stats_) (Variables|Default|GetDamage%20Dealt))))